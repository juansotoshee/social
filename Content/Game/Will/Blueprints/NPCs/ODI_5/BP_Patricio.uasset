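; BP_Patricio is an NPC that reacts to dialogue choices and can start an example cutscene when talked to.
; Construction creates a dynamic body material, which dialogue option strings recolour green, red or blue.
; Other options activate a referenced item or remove a Key from the player's inventory.
; TalkTo triggers the overview scene manager's cutscene for CutsceneDialogue, then defers to the parent; a helper updates walk speed.
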(event EventBeginPlay)

(event Collision|EventActorBeginOverlap
  (params (OtherActor :type Actor%20Object%20Reference)))

(event EventTick
  (params (DeltaSeconds :type Float%20%28single-precision%29))
  (|CallParentFunction DeltaSeconds))

(fn ConstructionScript
  (|CallParentFunction)
  (bind _returnvalue (Rendering|Material|CreateDynamicMaterialInstance (Variables|Character|GetMesh) 0 "/Game/PNCTookit/PNCGame/Characters/Mannequin3D/Character/Materials/MI_Man_Body_02_Inst.MI_Man_Body_02_Inst" "None" :!class /Script/Engine.PrimitiveComponent))
  (Variables|Default|SetMeshColourMID _returnvalue))

(fn OnReturnDialogueOption
  (params (ReturnOption :type String))
  ;[1 0.9481 0.4248 0.3] Run the following functionality when a valid dialogue option string is returned.
  (switch string ReturnOption
    (:Colour_Green
      (Rendering|Material|SetVectorParameterValue (Variables|Default|GetMeshColourMID) "BodyColor" "(R=0.052083,G=1.000000,B=0.067310,A=1.000000)" :!class /Script/Engine.MaterialInstanceDynamic))
    (:Colour_Red
      (Rendering|Material|SetVectorParameterValue (Variables|Default|GetMeshColourMID) "BodyColor" "(R=1.000000,G=0.000000,B=0.012731,A=1.000000)" :!class /Script/Engine.MaterialInstanceDynamic))
    (:Colour_Blue
      (Rendering|Material|SetVectorParameterValue (Variables|Default|GetMeshColourMID) "BodyColor" "(R=0.010417,G=0.213687,B=1.000000,A=1.000000)" :!class /Script/Engine.MaterialInstanceDynamic))
    (:Spawn.Key
      (Default|SetItemActiveState (Variables|Default|GetItemRef) true))
    (:Remove.Player.Item.Key
      (Default|RemoveInventoryItem (Variables|/Game/PNCTookit/Blueprints/BP_PNCPlayerController.BP_PNCPlayerController_C|GetInventoryComponent (CallFunction|GetPNCPlayerController)) "Key" false)))
  (return true))

(fn Talkto
  (params (Instigator :type Actor%20Object%20Reference) (Dialogue :type Name :default "None"))
  (if (Utilities|Name|Equal(Name) (Variables|Default|GetInteractionDialogue) "CutsceneDialogue")
    ;[1 1 1] Custom example cutscene when the player talks to this NPC.
    (bind _asbp_overview_scene_manager (Utilities|Casting|CastToBP_OverviewSceneManager (CallFunction|GetSceneManager))
      (:then
        (Default|BeginExampleCutscene _asbp_overview_scene_manager)
        (bind _success (|CallParentFunction 0 "None"))
        (return _success))
      (:CastFailed
        (return false)))
    (else
      (bind _success_2 (|CallParentFunction 0 "None"))
      (return _success_2))))

(fn UpdateWalkSpeed
  (params (NewWalkSpeed :type Float%20%28single-precision%29))
  (Variables|/Script/Engine.CharacterMovementComponent|SetMaxWalkSpeed (Variables|Character|GetCharacterMovement) NewWalkSpeed))