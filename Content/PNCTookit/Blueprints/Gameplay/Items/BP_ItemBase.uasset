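; Base Blueprint for pickup items that loads its data by item name from the Scene Manager's active item list shortly after BeginPlay.
; Pickup retries failed initialization, removes the item from its owning inventory, optionally starts dialogue and fires a pickup callback.
; Single-use items scale and glide toward the instigator on a timeline, then become hidden and non-colliding.
; Construction generates a GUID for save games, and inspection can trigger dialogue.
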(event Custom|PlayPickupAnim
  (params (Actor :type Actor%20Object%20Reference))
  ;[0.3083 0.7875 1 0.3] Play pickup animation
  (Variables|System|SetScaleTemp (Transformation|GetActorScale3D))
  (bind _scale (Timeline|Pickup_Timeline PlayFromStart)
    (:Update
      (Utilities|IsValid Actor
        (:Is%20Valid
          (Transformation|SetActorLocation (Math|Interpolation|VInterpTo (Transformation|GetActorLocation) (Transformation|GetActorLocation Actor) (Utilities|Time|GetWorldDeltaSeconds) 1e+01) false false))
        (:Is%20Not%20Valid
          _))
      (Transformation|SetActorScale3D (* (Variables|System|GetScaleTemp) _scale)))
    (:Finished
      (CallFunction|SetItemActiveState false))))

(event EventBeginPlay
  ;[0.3083 0.7875 1 0.3] Begin Play - Init and Set item save state
  (Utilities|FlowControl|Delay 0.1) ; Short delay before load
  (CallFunction|Init)
  (CallFunction|SetItemActiveState (Variables|System|GetbIsActive)) ; Set item save state
)

(fn ConstructionScript
  ;[0.4913 0.6396 1 0.3] If not valid, generate a new unique identifier for this interactive actor instance. Used for Save Games.
  (Default|GenerateGUID (Variables|Default|GetGlobalInteractionComponent) false))

(fn SetItemActiveState
  (params (bActive :type Boolean))
  ;[1 0.9161 0.3541 0.3] Set the visibility and interaction state of the item.
  (bind _output_get (Variables|System|SetbIsActive bActive))
  (if _output_get
    (Rendering|SetActorHiddenInGame false)
    (Collision|SetActorEnableCollision true)
    (else
      (Rendering|SetActorHiddenInGame true)
      (Collision|SetActorEnableCollision false)))
  (return true))

(fn SetItemData
  ;[0.3869 1 0.9 0.3] Set Item Data
  (bind (_returnvalid _itemdata) (CallFunction|GetItemData (Variables|ItemData|GetItemName)))
  (if _returnvalid
    (Variables|ItemData|SetItemDataStruct _itemdata)
    (Variables|System|SetbIsInitialized true)
    (return true)
    (else
      (Variables|System|SetbIsInitialized false)
      (CallFunction|CustomPrint (Utilities|String|Append "Failed to find \"" (Utilities|String|ToString(Name) (Variables|ItemData|GetItemName)) "\" item in the Scene Managers Active Item List. Unable to Initialize.") "NewEnumerator4" false)
      (return false))))

(fn RemoveItemfromParentInventory
  (bind _itemowningparent (Variables|System|GetItemOwningParent)
    (:then
      (Utilities|IsValid (Actor|GetComponentbyClass _itemowningparent "/Game/PNCTookit/Blueprints/Components/BP_InventoryComponent.BP_InventoryComponent_C")
        (:Is%20Valid
          (Default|RemoveInventoryItem (Actor|GetComponentbyClass _itemowningparent "/Game/PNCTookit/Blueprints/Components/BP_InventoryComponent.BP_InventoryComponent_C") (Variables|ItemData|GetItemName) false))))
    (:else)))

(fn Init
  ;[0.436 0.9602 1 0.3] Initialize item data
  (CallFunction|SetItemData))

(fn GetItemName
  (return (Variables|ItemData|GetItemName)))

(fn IsInventoryItem
  (return true))

(fn OnInspection
  (params (Inspector :type Controller%20Object%20Reference))
  (if (Utilities|Name|NotEqual(Name) (Variables|Settings|GetOnInspectionDialogue) "None")
    (CallFunction|StartDialogueSequence (Variables|Settings|GetOnInspectionDialogue) self)
    (return true)
    (else
      (return false))))

(fn Pickup
  (params (Instigator :type Actor%20Object%20Reference))
  ;[0.3957 1 0.9901 0.3] On pickup set the new state (if any change) to the item.
  (if (Variables|System|GetbIsInitialized)
    _
    (else
      ;;[1 0.8796 0.2086 0.298] Update 1.1 - Extra warnings when items fail to initialize
      (CallFunction|Init) ; Retry Initialization if it had failed on startup.
      (if (Variables|System|GetbIsInitialized)
        _
        (else
          (CallFunction|CustomPrint (Utilities|String|Append "Failed to find \"" (Utilities|String|ToString(Name) (Variables|ItemData|GetItemName)) "\" item in the Scene Managers Active Item List. Aborting pickup action.") "NewEnumerator4" false)
          (return false)))))
  (if (Variables|System|GetbIsActive)
    (if (Variables|Settings|GetbSingleUse)
      (Variables|System|SetbIsActive false)
      (CallFunction|PlayPickupAnim (Variables|Actor|GetInstigator))
      (Collision|SetActorEnableCollision false))
    (CallFunction|RemoveItemfromParentInventory)
    (if (Utilities|Name|NotEqual(Name) (Variables|Settings|GetOnPickupDialogue) "None")
      (CallFunction|StartDialogueSequence (Variables|Settings|GetOnPickupDialogue)))
    (Default|CallOnPickup)
    (return true)
    (else
      (return false))))

(fn RecieveItem
  (params (ItemName :type Name :default "None"))
  (return false false))

(fn UseObject
  (params (InteractingCharacter :type BP%20PNC%20Character%20Parent%20Object%20Reference))
  (return false))