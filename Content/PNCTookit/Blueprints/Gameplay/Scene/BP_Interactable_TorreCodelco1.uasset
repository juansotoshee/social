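; Interactable tower object that accepts the "Pasarela" inventory item, then reveals a block, raises it and marks itself used.
; A timeline lerps the block from its starting location to the Box component's location at a configurable play rate.
; During the move it disables player input and cuts to CameraTC1.
; A three-second delay triggered from the timeline update then blends back to the PNC camera manager and re-enables input.
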(event Custom|Move%20Up%20Anim
  (Default|SetInputEnabled (CallFunction|GetPNCPlayerController) false)
  (Game|Player|SetViewTargetwithBlend (CallFunction|GetPNCPlayerController) (Variables|Default|GetcameraTC1) 0.0 "VTBlend_Linear" 0.0 false)
  (bind _pos (Timeline|Up%20Timeline Play)
    (:Update
      (Transformation|SetWorldLocation (Variables|Default|Getblock) (Math|Vector|Lerp(Vector) (Variables|Default|GetstartLocation) (Variables|Default|GetendLocation) _pos) false false)
      (Utilities|FlowControl|Delay 3.0)
      (Game|Player|SetViewTargetwithBlend (CallFunction|GetPNCPlayerController) (CallFunction|GetPNCCameraManager) 1.0 "VTBlend_EaseInOut" 5.0 false)
      (Default|SetInputEnabled (CallFunction|GetPNCPlayerController) true))))

(event EventBeginPlay
  (|CallParentFunction)
  (Variables|Default|SetstartLocation (Transformation|GetWorldLocation (Variables|Default|Getblock)))
  (Variables|Default|SetendLocation (Transformation|GetWorldLocation (Variables|Default|GetBox)))
  (Components|Timeline|SetPlayRate (Variables|Default|GetUp%20Timeline) (Variables|Default|GetplayRate)))

(fn ConstructionScript
  (|CallParentFunction))

(fn OnInspection
  (params (Inspector :type Controller%20Object%20Reference))
  (return false))

(fn GetItemName
  (return "None"))

(fn IsInventoryItem
  (return false))

(fn Pickup
  (params (Instigator :type Actor%20Object%20Reference))
  (return false))

(fn RecieveItem
  (params (ItemName :type Name :default "None"))
  (switch name ItemName
    (:Default
      (return false false))
    (:Pasarela
      (Rendering|SetVisibility (Variables|Default|Getblock) true false)
      (CallFunction|MoveUpAnim)
      (Variables|Default|SetbIsUsed true)
      (return true true))))