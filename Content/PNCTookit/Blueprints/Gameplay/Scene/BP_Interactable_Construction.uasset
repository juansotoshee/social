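; BP_Interactable_Construction is a point-and-click scene interactable that turns into a walkway when given the Pasarela item.
; RecieveItem switches on the item name: Pasarela hides the Cube, shows the Pasarela component, sets IsUsed and reports the item valid and consumed.
; Any other item is rejected, and the inspection, pickup and inventory functions all return false.
; The event graph holds only disabled default nodes.
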(event EventBeginPlay
  (|CallParentFunction) ; This node is disabled and will not be called.\nDrag off pins to build functionality.
)

(event Collision|EventActorBeginOverlap
  (params (OtherActor :type Actor%20Object%20Reference)))

(event EventTick
  (params (DeltaSeconds :type Float%20%28single-precision%29)))

(fn ConstructionScript
  (|CallParentFunction))

(fn OnInspection
  (params (Inspector :type Controller%20Object%20Reference))
  (return false))

(fn GetItemName
  (return "None"))

(fn IsInventoryItem
  (return false))

(fn Pickup
  (params (Instigator :type Actor%20Object%20Reference))
  (return false))

(fn RecieveItem
  (params (ItemName :type Name :default "None"))
  (switch name ItemName
    (:Default
      (return false false))
    (:Pasarela
      (Rendering|SetVisibility (Variables|Default|GetCube) false false)
      (Rendering|SetVisibility (Variables|Default|GetPasarela) true false)
      (Variables|Default|SetbIsUsed true)
      (return true true))))