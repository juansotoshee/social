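; Visual door actor that layers open, close and locked feedback onto its parent's enter and exit logic.
; Successful enter or exit plays a timeline that swings the door mesh, optionally flipped; failed attempts on a locked door rotate the lock mesh.
; When the last moving character completes, a retriggerable delay reverses the swing to close the door.
; Lock mesh visibility follows the unlocked state at construction, on BeginPlay and on state changes.
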(event Custom|CloseDoor
  ;[0.4233 1 0.4072 0.298] Comment
  (Utilities|FlowControl|RetriggerableDelay (Variables|Settings|GetCloseDelay)) ; Close Door after delay
  (bind (_direction _door_rotation) (Timeline|Open%20Door%20Anim Reverse)
    (:Update
      (Transformation|SetRelativeRotation (Variables|Default|GetDoorMesh) (Math|Rotator|MakeRotator 0.0 0.0 (select (Variables|Default|GetbFlipOpenDirection) (* _door_rotation -1.0) _door_rotation)) false false))
    (:Finished
      (switch Utilities|FlowControl|Switch|SwitchonETimelineDirection _direction
        (:Forward
          (Variables|Default|SetbDoorOpen true))
        (:Backward
          (Variables|Default|SetbDoorOpen false))))))

(event Custom|OpenDoor
  ;[0.4233 1 0.4072 0.298] Comment
  (bind (_direction _door_rotation) (Timeline|Open%20Door%20Anim Play)
    (:Update
      (Transformation|SetRelativeRotation (Variables|Default|GetDoorMesh) (Math|Rotator|MakeRotator 0.0 0.0 (select (Variables|Default|GetbFlipOpenDirection) (* _door_rotation -1.0) _door_rotation)) false false))
    (:Finished
      (switch Utilities|FlowControl|Switch|SwitchonETimelineDirection _direction
        (:Forward
          (Variables|Default|SetbDoorOpen true))
        (:Backward
          (Variables|Default|SetbDoorOpen false))))))

(event Custom|OnEnterFailed
  ;[0.4233 1 0.4072 0.298] Comment
  (if (and (not (Variables|Default|GetbIsUnlocked)) (not (Audio|Components|Audio|IsPlaying (Variables|Default|GetDoor%20Locked%20Anim))))
    (bind _door_rotation (Timeline|Door%20Locked%20Anim PlayFromStart)
      (:Update
        (Transformation|SetRelativeRotation (Variables|Default|GetLockMesh) (Math|Rotator|MakeRotator 0.0 _door_rotation 0.0) false false)))))

(event EventBeginPlay
  ;[1 1 1] Set Current locked state on load.
  (CallFunction|ChangeDoorLockedState (Variables|Default|GetbIsUnlocked)))

(fn ConstructionScript
  (|CallParentFunction)
  (Rendering|SetVisibility (Variables|Default|GetLockMesh) (not (Variables|Default|GetbIsUnlocked)) false))

(fn EnterDoor
  (params (EnteringCharacter :type BP%20PNC%20Character%20Parent%20Object%20Reference))
  (bind _success (|CallParentFunction EnteringCharacter))
  (if _success
    (CallFunction|OpenDoor)
    (else
      (CallFunction|OnEnterFailed)))
  (return _success))

(fn ExitDoor
  (params (Character :type BP%20PNC%20Character%20Parent%20Object%20Reference))
  (bind _success (|CallParentFunction Character))
  (if _success
    (CallFunction|OpenDoor)
    (else
      (CallFunction|OnEnterFailed)))
  (return _success))

(fn OnCharacterMoveCompletion
  (params (Character :type BP%20PNC%20Character%20Parent%20Object%20Reference))
  (bind _value (CallFunction|GetCharacterMapping Character))
  ;[0.4233 1 0.4072 0.298] If the character has successfully moved to the Indoor or Outdoor location, check to see if the door can be closed. If there are still multiple characters moving In/out of the door, then wait for them to complete before closing
  (if (or (Utilities|Enum|Equal(Enum) _value "NewEnumerator0") (Utilities|Enum|Equal(Enum) _value "NewEnumerator1"))
    (Utilities|FlowControl|Sequence
      (:then_0
        (if (>= (Utilities|Map|Length (Variables|Default|GetCharacterBindings)) 2) ; Is this the last character moving in/out of the door?
          (return false)
          (else
            (CallFunction|CloseDoor))))
      (:then_1
        (|CallParentFunction Character :!label _label)
        (return false)))
    (else
      (goto _label))))

(fn ChangeDoorLockedState
  (params (Unlocked :type Boolean))
  (bind _return (|CallParentFunction Unlocked))
  (if Unlocked
    (Rendering|SetVisibility (Variables|Default|GetLockMesh) false false)
    (else
      (Rendering|SetVisibility (Variables|Default|GetLockMesh) true false)))
  (return _return))