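; Base Blueprint for interactable scene objects, giving child classes saved state plus use and inspection hooks.
; The construction script has GlobalInteractionComponent generate a GUID if invalid, identifying each instance for save games.
; BeginPlay calls Init, which loads the object state, then runs LoadGameplayState for children to apply it; children using BeginPlay must call parent.
; Children override OnInspection, a logging stub here, and UseObject, which returns IsActive.
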(event EventBeginPlay
  ;[1 0.8991 0.2581 0.3] Initialize the interactable object when brought into the world.
  ;
  ; Note: If you use "Event Begin Play" in your child classes, be sure to also "Add Call to Parent" before doing anything else. If this isnt done, init wont be called and the object state may not load/ be setup properly and cause issues.
  (CallFunction|Init))

(fn ConstructionScript
  ;[0.4913 0.6396 1 0.3] If not valid, generate a new unique identifier for this interactive actor instance. Used for Save Games.
  (Default|GenerateGUID (Variables|Default|GetGlobalInteractionComponent) false))

(fn Init
  ;[0.2916 0.7981 1 0.3] Load interactable object state
  (bind _return (CallFunction|LoadInteractableObjectState self))
  (if _return
    _
    (else
      _))
  (CallFunction|LoadGameplayState))

(fn LoadGameplayState
  ;[1 0.7171 0.2353 0.3] Override this function in all interactable object child classes.
  ;
  ; While the "Init" function is used to load the "object" state,   this function will use the object state data (e.g. IsActive or IsUsed) to load the custom "gameplay" state of the object.
  ;
  ; For example, if one of the light objects in the scene had "IsUsed" set to 'true', this "Load Gameplay State" function will then set the light as visible in the scene.
  (return true))

(fn OnInspection
  (params (Inspector :type Controller%20Object%20Reference))
  ;[1 0.9411 0.3122 0.3] Override this in children classes to handle inspection dialogue/functionality
  (CallFunction|CustomPrint "Inspecting Actor.  Override \"On Inspection\" interface function in the child blueprint." "NewEnumerator3" false)
  (return false))

(fn UseObject
  (params (InteractingCharacter :type BP%20PNC%20Character%20Parent%20Object%20Reference))
  ;[1 0.5293 0.7243 0.3] Children should override this function but still call it to see whether or not the object is currently active.
  (return (Variables|ObjectState|GetbIsActive)))