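; Blueprint function library of save-game helpers that capture and look up character and scene state for the PNC Toolkit.
; Gather functions build save structs from characters, player controller, items, doors, interactables and scene state strings, tagged with GUIDs from each actor's Global Interaction Component.
; Lookup functions read the autosave slot to find characters by GUID or scenes by name, returning found/valid flags.
; Small utilities supply the autosave slot name and an unused numbered slot.
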(fn GetCharacterStructinArray
  (params (CharacterName :type String) (GUID :type Guid%20Structure))
  ;[0.4825 0.6541 1 0.3] Return the latest character saves state (struct)
  (bind _savegame (CallFunction|CreateorLoadSaveGame (CallFunction|GetGameSlot true) false))
  (Utilities|IsValid _savegame
    (:Is%20Valid
      (for (_array_element _array_index) (Variables|/Game/PNCTookit/Blueprints/SaveGame/BP_PNCSaveGame.BP_PNCSaveGame_C|GetCharacterArray _savegame)
        (if (== (Utilities|Struct|BreakSCharacterSave _array_element) GUID)
          (return _array_element true _array_index)))
      (CallFunction|CustomPrint (Utilities|String|Append "Unable to find \"" CharacterName "\" in Character Array. ") "NewEnumerator0" true))
    (:Is%20Not%20Valid
      _))
  (return "" false -1))

(fn GetAutoSaveGameSlotName
  ;[1 0.4532 0.9055 0.3] Returns the name of the Autosave slot created when the client begins, and removed when the client is closed
  (return "Autosave"))

(fn GetCharacterState
  (params (Actor :type Actor%20Object%20Reference))
  (LocalVariables|SetActorRef Actor)
  (LocalVariables|SetName (Utilities|GetObjectName (LocalVariables|GetActorRef)))
  (bind _output_get (LocalVariables|SetGlobalInteractionComponentRef (Actor|GetComponentbyClass (LocalVariables|GetActorRef) "/Game/PNCTookit/Blueprints/Components/BP_GlobalInteractionComponent.BP_GlobalInteractionComponent_C")))
  (Utilities|IsValid _output_get
    (:Is%20Valid
      ;[0.959 0.6731 1 0.3] If the actor has an inventory component, get the inventory
      (Utilities|IsValid (Actor|GetComponentbyClass (LocalVariables|GetActorRef) "/Game/PNCTookit/Blueprints/Components/BP_InventoryComponent.BP_InventoryComponent_C") ; Does the Character have an Inventory component?
        (:Is%20Valid
          (LocalVariables|SetInventory (Default|GetInventory (Actor|GetComponentbyClass (LocalVariables|GetActorRef) "/Game/PNCTookit/Blueprints/Components/BP_InventoryComponent.BP_InventoryComponent_C"))))
        (:Is%20Not%20Valid
          _))
      (bind _asbp_pnccharacter_parent (Utilities|Casting|CastToBP_PNCCharacter_Parent (LocalVariables|GetActorRef))
        (:then
          ;[0.959 0.6731 1 0.3] Return Save struct for Character
          (return (Utilities|Struct|MakeSCharacterSave (Variables|/Game/PNCTookit/Blueprints/Components/BP_GlobalInteractionComponent.BP_GlobalInteractionComponent_C|GetGUID (LocalVariables|GetGlobalInteractionComponentRef)) (LocalVariables|GetName) (LocalVariables|GetInventory) (Transformation|GetActorTransform (LocalVariables|GetActorRef)) (Variables|/Game/PNCTookit/Blueprints/Characters/BP_PNCCharacter_Parent.BP_PNCCharacter_Parent_C|GetbIsSpokenTo _asbp_pnccharacter_parent))))
        (:CastFailed
          (Utilities|Casting|CastToBP_PNCPlayerController (LocalVariables|GetActorRef)
            (:then
              ;[0.959 0.6731 1 0.3] Return Save struct for Player Controller
              (return (Utilities|Struct|MakeSCharacterSave (Variables|/Game/PNCTookit/Blueprints/Components/BP_GlobalInteractionComponent.BP_GlobalInteractionComponent_C|GetGUID (LocalVariables|GetGlobalInteractionComponentRef)) (LocalVariables|GetName) (LocalVariables|GetInventory) (Transformation|GetActorTransform (LocalVariables|GetActorRef)) true)))
            (:CastFailed
              ;[1 0.1875 0.1875 0.3] Failed to return save struct for character based on the actor
              (CallFunction|CustomPrint (Utilities|String|Append "Failed to save Get Character Save struct for \" " (Utilities|GetDisplayName (LocalVariables|GetActorRef)) " \" ") "NewEnumerator5" true)
              (return ""))))))
    (:Is%20Not%20Valid
      (CallFunction|CustomPrint (Utilities|String|Append (Utilities|GetDisplayName (LocalVariables|GetActorRef)) " does not contain a Global Interaction Component. Actor cant be  saved. ") "NewEnumerator0" true)
      (return ""))))

(fn GetSceneStateStrings
  (bind _return (CallFunction|GetSceneManager))
  ;[1 0.5948 0.9057 0.3] Return a list of the current scenes "State strings"
  (Utilities|IsValid _return
    (:Is%20Valid
      (return (Variables|/Game/PNCTookit/Blueprints/BP_SceneManagerBase.BP_SceneManagerBase_C|GetStateAsStrings _return)))
    (:Is%20Not%20Valid
      (return 0))))

(fn GetSceneItemsState
  ;[0.7812 0.5625 1 0.3] Return all current state of each item in the level
  (bind _outactors (Actor|GetAllActorsOfClass 0 "/Game/PNCTookit/Blueprints/Gameplay/Items/BP_ItemBase.BP_ItemBase_C"))
  (for _array_element _outactors
    (if (not (Variables|/Game/PNCTookit/Blueprints/Gameplay/Items/BP_ItemBase.BP_ItemBase_C|GetbRespawnOnSceneLoad _array_element))
      (Utilities|Array|Add (LocalVariables|GetItemsArray) (Utilities|Struct|MakeSItemsState (Variables|/Game/PNCTookit/Blueprints/Components/BP_GlobalInteractionComponent.BP_GlobalInteractionComponent_C|GetGUID (Variables|/Game/PNCTookit/Blueprints/Gameplay/Items/BP_ItemBase.BP_ItemBase_C|GetGlobalInteractionComponent _array_element)) (Utilities|GetObjectName _array_element) (Variables|/Game/PNCTookit/Blueprints/Gameplay/Items/BP_ItemBase.BP_ItemBase_C|GetbIsActive _array_element)))))
  (return (LocalVariables|GetItemsArray)))

(fn GetSceneDoorsState
  ;[0.5521 1 0.5154 0.33] Return the state of each Door actor within the scene
  (bind _outactors (Actor|GetAllActorsOfClass 0 "/Game/PNCTookit/Blueprints/Gameplay/Scene/BP_DoorBase.BP_DoorBase_C"))
  (for _array_element _outactors
    (Utilities|Array|Add (LocalVariables|GetDoorStateArray) (Utilities|Struct|MakeSDoorState (Variables|/Game/PNCTookit/Blueprints/Components/BP_GlobalInteractionComponent.BP_GlobalInteractionComponent_C|GetGUID (Variables|/Game/PNCTookit/Blueprints/Gameplay/Scene/BP_DoorBase.BP_DoorBase_C|GetGlobalInteractionComponent _array_element)) (Utilities|GetObjectName _array_element) (Variables|/Game/PNCTookit/Blueprints/Gameplay/Scene/BP_DoorBase.BP_DoorBase_C|GetbIsUnlocked _array_element))))
  (return (LocalVariables|GetDoorStateArray)))

(fn GetSceneStatebyName
  (params (SceneName :type String))
  ;[0.4989 0.8272 1 0.3] Finds and returns a scenes save struct (If Valid).
  ;
  ; This can be used to get and modify the state of a scene even when it is not currently active ingame (For example, saving state strings for scenes that are currently not opened).
  ; This is mostly paired up with SaveSceneState function.
  ;
  ; Note: Keep in mind, un-saved scenes can either be created and return as valid, OR have a new scene generated and return as an invalid scene
  (LocalVariables|SetSceneNameRef SceneName)
  (bind _savegame (CallFunction|CreateorLoadSaveGame (CallFunction|GetGameSlot true) false))
  (Utilities|IsValid _savegame
    (:Is%20Valid
      (if (>= (Utilities|Array|Length (Variables|/Game/PNCTookit/Blueprints/SaveGame/BP_PNCSaveGame.BP_PNCSaveGame_C|GetSceneList _savegame)) 1)
        (if (Utilities|Array|ContainsItem (Variables|/Game/PNCTookit/Blueprints/SaveGame/BP_PNCSaveGame.BP_PNCSaveGame_C|GetSceneList _savegame) (LocalVariables|GetSceneNameRef))
          (return (Utilities|Array|Get(acopy) (Utilities|Struct|BreakSGlobalSceneList (Variables|/Game/PNCTookit/Blueprints/SaveGame/BP_PNCSaveGame.BP_PNCSaveGame_C|GetSceneStructArray _savegame)) (Utilities|Array|FindItem (Variables|/Game/PNCTookit/Blueprints/SaveGame/BP_PNCSaveGame.BP_PNCSaveGame_C|GetSceneList _savegame) (LocalVariables|GetSceneNameRef))) true)
          (else
            _))))
    (:Is%20Not%20Valid
      _))
  (return "" false))

(fn GetAllInteractableObjectStates
  ;[0.3747 0.6875 1 0.3] Collects and returns the state of all interactable objects within the scene via a single struct.
  ; Note: This is mainly used when saving the state of the scene.
  (bind _outactors (Actor|GetAllActorsOfClass 0 "/Game/PNCTookit/Blueprints/Gameplay/Scene/BP_InteractableObjectBase.BP_InteractableObjectBase_C"))
  (for _array_element _outactors
    (bind _output_get (LocalVariables|SetLoopInteractableObject _array_element))
    (Utilities|Array|AddUnique (LocalVariables|GetList) (Utilities|GetObjectName _output_get))
    (Utilities|IsValid (Actor|GetComponentbyClass (LocalVariables|GetLoopInteractableObject) "/Game/PNCTookit/Blueprints/Components/BP_InventoryComponent.BP_InventoryComponent_C") ; Does the Interactable Object  have an Inventory component?
      (:Is%20Valid
        (Utilities|Array|Add (LocalVariables|GetInteractableObjectStates) (Utilities|Struct|MakeSInteractableObjectState (Variables|/Game/PNCTookit/Blueprints/Components/BP_GlobalInteractionComponent.BP_GlobalInteractionComponent_C|GetGUID (Variables|/Game/PNCTookit/Blueprints/Gameplay/Scene/BP_InteractableObjectBase.BP_InteractableObjectBase_C|GetGlobalInteractionComponent (LocalVariables|GetLoopInteractableObject))) (Utilities|GetObjectName (LocalVariables|GetLoopInteractableObject)) (Variables|/Game/PNCTookit/Blueprints/Gameplay/Scene/BP_InteractableObjectBase.BP_InteractableObjectBase_C|GetbIsActive (LocalVariables|GetLoopInteractableObject)) (Variables|/Game/PNCTookit/Blueprints/Gameplay/Scene/BP_InteractableObjectBase.BP_InteractableObjectBase_C|GetbIsUsed (LocalVariables|GetLoopInteractableObject)) (Default|GetInventory (Actor|GetComponentbyClass (LocalVariables|GetLoopInteractableObject) "/Game/PNCTookit/Blueprints/Components/BP_InventoryComponent.BP_InventoryComponent_C")))))
      (:Is%20Not%20Valid
        (Utilities|Array|Add (LocalVariables|GetInteractableObjectStates) (Utilities|Struct|MakeSInteractableObjectState (Variables|/Game/PNCTookit/Blueprints/Components/BP_GlobalInteractionComponent.BP_GlobalInteractionComponent_C|GetGUID (Variables|/Game/PNCTookit/Blueprints/Gameplay/Scene/BP_InteractableObjectBase.BP_InteractableObjectBase_C|GetGlobalInteractionComponent (LocalVariables|GetLoopInteractableObject))) (Utilities|GetObjectName (LocalVariables|GetLoopInteractableObject)) (Variables|/Game/PNCTookit/Blueprints/Gameplay/Scene/BP_InteractableObjectBase.BP_InteractableObjectBase_C|GetbIsActive (LocalVariables|GetLoopInteractableObject)) (Variables|/Game/PNCTookit/Blueprints/Gameplay/Scene/BP_InteractableObjectBase.BP_InteractableObjectBase_C|GetbIsUsed (LocalVariables|GetLoopInteractableObject)) (Utilities|Map|MakeMap "None" ""))))))
  (return (Utilities|Struct|MakeSInteractableObjectList (LocalVariables|GetList) (LocalVariables|GetInteractableObjectStates))))

(fn GetUnusedSaveGameName
  ;[1 0.9221 0.4062 0.3] Find a save game "Slot" name not currently in use
  (for _index (range 0 100)
    (bind _returnvalue (SaveGame|DoesSaveGameExist (Utilities|String|Append "Slot" (Utilities|String|ToString(Integer) _index))))
    (if (not _returnvalue)
      (return (Utilities|String|Append "Slot" (Utilities|String|ToString(Integer) _index)))))
  (CallFunction|CustomPrint "You have created way to many saves!  (100) " "NewEnumerator4" true)
  (return "MAXCAPSAve"))