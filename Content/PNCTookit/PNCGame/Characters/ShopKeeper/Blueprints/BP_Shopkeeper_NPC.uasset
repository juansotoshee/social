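; Shopkeeper NPC that gives and completes the rubbish-collecting quest in a point-and-click game.
; A dialogue option starts the quest by adding a scene state string, which TalkTo checks to choose the conversation.
; With enough ripped pages, TalkTo marks the quest completed, swaps the pages for a Match (a comment says Flint) and plays completion dialogue.
; Later talks get short post-quest dialogue; other cases fall back to the parent's dialogue.
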(event EventBeginPlay)

(event Collision|EventActorBeginOverlap
  (params (OtherActor :type Actor%20Object%20Reference)))

(event EventTick
  (params (DeltaSeconds :type Float%20%28single-precision%29))
  (|CallParentFunction DeltaSeconds))

(fn ConstructionScript
  (|CallParentFunction))

(fn OnReturnDialogueOption
  (params (ReturnOption :type String))
  (switch string ReturnOption
    (:Default
      (return false))
    (:BeginRubbishQuest
      (Default|AddStateStringtoScene (CallFunction|GetSceneManager) "" "RubbishQuest")
      (return true))))

(fn Talkto
  (params (Instigator :type Actor%20Object%20Reference) (Dialogue :type Name :default "None"))
  (bind _return (CallFunction|GetSceneManager))
  (bind _controller (CallFunction|GetPNCPlayerController))
  (bind _return_2 (CallFunction|GetSceneManager))
  (bind _return_3 (Default|GetStateStrings _return))
  (bind _inventorycomponent (Variables|/Game/PNCTookit/Blueprints/BP_PNCPlayerController.BP_PNCPlayerController_C|GetInventoryComponent _controller))
  (if (Utilities|Array|ContainsItem _return_3 "RubbishQuest")
    ;[1 0.7459 0.4961 0.3] If the player successfully collects all 8 pages in the scene, remove the quest and page items from the players inventory. Add the "Flint" item to the players inventory.
    (bind _return_4 (CallFunction|ConditionHasIteminInventory (CallFunction|GetPNCPlayerController) "RippedPage" 8))
    (if _return_4
      (Default|RemoveStateStringfromScene _return_2 "" "RubbishQuest")
      (Default|AddStateStringtoScene _return_2 "" "CompletedRubbishQuest")
      (Default|AddInventoryItem _inventorycomponent "Match")
      (Default|RemoveInventoryItem _inventorycomponent "RippedPage" true)
      (CallFunction|StartDialogueSequence "TalkToShopKeeperQuestComplete" self)
      (return true)
      (else
        _))
    (elif (Utilities|Array|ContainsItem _return_3 "CompletedRubbishQuest")
      ;[1 0.6583 0.9569 0.3] Short dialogue if the player talks to the shopkeeper when they have already completed the quest
      (CallFunction|StartDialogueSequence "TalkToShopKeeperQuestCompleted" self)
      (return true)
      (else
        _)))
  ;[0.4909 1 0.4973 0.3] Standard dialogue when spoken to during quest.
  (bind _success (|CallParentFunction (Variables|Default|GetInstigator) Dialogue))
  (return _success))