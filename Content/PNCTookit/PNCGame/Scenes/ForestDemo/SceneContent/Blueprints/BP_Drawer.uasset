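; Interactive drawer for the forest demo that toggles open and closed when a character uses it.
; A timeline blends the mesh toward configurable open location and rotation and reverses to close, with IsActive switched off when movement starts.
; The construction script snaps an optional referenced item to the PaperItemLocation component.
; Loading gameplay state replays the open animation if the drawer was used.
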(event Custom|PlayCloseAnim
  (Variables|Default|SetbIsActive false)
  (bind (_direction _locationalpha _rotationalpha) (Timeline|OpenCloseAnim Reverse)
    (:Update
      (Transformation|SetRelativeLocationAndRotation (Variables|Default|GetDrawerMesh) (Math|Vector|Lerp(Vector) "0, 0, 0" (Variables|Default|GetOpenLocation) _locationalpha) (Math|Rotator|Lerp(Rotator) "0, 0, 0" (Variables|Default|GetOpenRotation) _rotationalpha) false false))
    (:Finished
      (Variables|Default|SetbIsActive true))))

(event Custom|PlayOpenAnim
  (Variables|Default|SetbIsActive false)
  (bind (_direction _locationalpha _rotationalpha) (Timeline|OpenCloseAnim PlayFromStart)
    (:Update
      (Transformation|SetRelativeLocationAndRotation (Variables|Default|GetDrawerMesh) (Math|Vector|Lerp(Vector) "0, 0, 0" (Variables|Default|GetOpenLocation) _locationalpha) (Math|Rotator|Lerp(Rotator) "0, 0, 0" (Variables|Default|GetOpenRotation) _rotationalpha) false false))
    (:Finished
      (Variables|Default|SetbIsActive true))))

(fn ConstructionScript
  (|CallParentFunction)
  (Utilities|IsValid (Variables|Default|GetItemRef)
    (:Is%20Valid
      (Transformation|AttachComponentToComponent (Variables|Default|GetItemRef) (Variables|Default|GetPaperItemLocation) "None" "SnapToTarget" "SnapToTarget" "SnapToTarget" true))))

(fn UseObject
  (params (InteractingCharacter :type BP%20PNC%20Character%20Parent%20Object%20Reference))
  (bind _success (|CallParentFunction InteractingCharacter))
  (if _success
    (if (Variables|Default|GetbIsUsed)
      (Variables|Default|SetbIsUsed false)
      (CallFunction|PlayCloseAnim)
      (else
        (Variables|Default|SetbIsUsed true)
        (CallFunction|PlayOpenAnim))))
  (return _success))

(fn LoadGameplayState
  (if (Variables|Default|GetbIsUsed)
    (CallFunction|PlayOpenAnim))
  (return true))