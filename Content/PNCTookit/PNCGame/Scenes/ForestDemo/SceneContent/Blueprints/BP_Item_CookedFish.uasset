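; BP_Item_CookedFish is a non-inventory item in the Forest demo that makes the player character throw a cooked fish at a hedge on pickup.
; A successful parent Pickup triggers ThrowCookedFishAnim, which waits briefly and spawns BP_CookedFish_Physics above the character.
; SuggestProjectileVelocity computes an arc toward a point above HedgeRef, and the result is fed to the fish's ProjectileMovement through SetVelocityInLocalSpace.
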(event Custom|ThrowCookedFishAnim
  (bind _return (CallFunction|GetPNCCharacter))
  (bind _returnvalue (Transformation|GetActorLocation _return))
  (Utilities|FlowControl|Delay 0.5)
  (bind _returnvalue_2 (Game|SpawnActorfromClass "/Game/PNCTookit/PNCGame/Scenes/ForestDemo/SceneContent/Blueprints/BP_CookedFish_Physics.BP_CookedFish_Physics_C" (Math|Transform|MakeTransform (+ _returnvalue "0, 0,100.000000")) "Undefined" 0 0))
  (bind _tossvelocity (Class|GameplayStatics|BlueprintSuggestProjectileVelocity _returnvalue (+ (Transformation|GetActorLocation (Variables|Default|GetHedgeRef)) "0, 0,100.000000") 1e+03 -1.0 "DoNotTrace" 5.0 false false))
  (Game|Components|ProjectileMovement|SetVelocityinLocalSpace (Variables|/Game/PNCTookit/PNCGame/Scenes/ForestDemo/SceneContent/Blueprints/BP_CookedFish_Physics.BP_CookedFish_Physics_C|GetProjectileMovement _returnvalue_2) _tossvelocity))

(fn ConstructionScript
  (|CallParentFunction))

(fn IsInventoryItem
  (return false))

(fn Pickup
  (params (Instigator :type Actor%20Object%20Reference))
  (bind _success (|CallParentFunction Instigator))
  (if _success
    (CallFunction|ThrowCookedFishAnim))
  (return _success))