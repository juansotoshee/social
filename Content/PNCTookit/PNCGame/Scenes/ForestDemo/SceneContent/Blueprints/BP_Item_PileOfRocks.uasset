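; Pile-of-rocks item for the PNC ForestDemo scene that hands out rocks and reacts to items used on it.
; Pickup removes one Rock from its own inventory component, failing with dialogue if the player already holds one or none remain.
; RecieveItem consumes the Broken Leaver, toggles item active states and plays the PickupAxe dialogue.
; A Branch triggers its own dialogue but, like other items, is rejected.
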(fn ConstructionScript
  (|CallParentFunction))

(fn RecieveItem
  (params (ItemName :type Name :default "None"))
  (switch name ItemName
    (:Default
      _)
    (:BrokenLeaver
      (CallFunction|SetItemActiveState false)
      (CallFunction|SetItemActiveState true)
      (CallFunction|StartDialogueSequence "PickupAxe")
      (return true true))
    (:Branch
      (CallFunction|StartDialogueSequence "BranchAxe")))
  (return false false))

(fn Pickup
  (params (Instigator :type Actor%20Object%20Reference))
  (if (Default|HasIteminInventory (Variables|/Game/PNCTookit/Blueprints/BP_PNCPlayerController.BP_PNCPlayerController_C|GetInventoryComponent (CallFunction|GetPNCPlayerController)) "Rock") ; Does the player already have a "Rock" item \nin their inventory?
    _
    (elif (Default|HasIteminInventory (Variables|Default|GetBP_InventoryComponent) "Rock") ; Does the "Pile Of Rocks" item still have rocks remaining?\n(haha, max the player can take is 2)
      (bind _return (Default|RemoveInventoryItem (Variables|Default|GetBP_InventoryComponent) "Rock" false))
      (return _return)
      (else
        _)))
  (CallFunction|StartDialogueSequence "PickupRockFailed")
  (return false))