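; BP_FakeTrapDoor is an interactable trap door in the point-and-click forest demo that only pretends it can open.
; A successful parent UseObject call triggers PlayLockedAnim, which clears IsActive and runs a timeline that pitches the trap door mesh in a locked animation.
; When the timeline finishes, it restores IsActive and starts the UseTrapDoor dialogue sequence.
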(event Custom|PlayLockedAnim
  (Variables|Default|SetbIsActive false)
  (bind _rot (Timeline|LockedAnim PlayFromStart)
    (:Update
      (Transformation|SetRelativeRotation (Variables|Default|GetTrapDoorMesh) (Math|Rotator|MakeRotator 0.0 _rot 0.0) false false))
    (:Finished
      (Variables|Default|SetbIsActive true)
      (CallFunction|StartDialogueSequence "UseTrapDoor"))))

(fn ConstructionScript
  (|CallParentFunction))

(fn UseObject
  (params (InteractingCharacter :type BP%20PNC%20Character%20Parent%20Object%20Reference))
  (bind _success (|CallParentFunction InteractingCharacter))
  (if _success
    (CallFunction|PlayLockedAnim))
  (return _success))