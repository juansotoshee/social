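; BP_TreeCutout is an interactable hedge obstacle in the ForestDemo point-and-click scene, removed by using the Fire Stick on it.
; The stick is consumed, fire particles play, and after a delay SetHedgeState hides the mesh and disables collision.
; Inspecting it or offering the Axe starts dialogue, and it cannot be picked up.
; LoadGameplayState reapplies IsUsed to restore the burned or intact state.
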(event Custom|SetHedgeOnFire
  (Components|Activation|Activate (Variables|Default|GetFireParticle) false)
  (Utilities|FlowControl|Delay 3.0)
  (CallFunction|SetHedgeState true)
  (Utilities|FlowControl|Delay 0.5)
  (Components|Activation|Deactivate (Variables|Default|GetFireParticle)))

(fn ConstructionScript
  (|CallParentFunction))

(fn SetHedgeState
  (params (bIsUsed :type Boolean))
  (Variables|Default|SetbIsUsed bIsUsed)
  (Development|SetHiddeninGame (Variables|Default|GetTreeCutoutMesh) (Variables|Default|GetbIsUsed) false)
  (Collision|SetActorEnableCollision (not (Variables|Default|GetbIsUsed))))

(fn OnInspection
  (params (Inspector :type Controller%20Object%20Reference))
  (CallFunction|StartDialogueSequence "InspectTreeCutout" Inspector)
  (return true))

(fn LoadGameplayState
  (CallFunction|SetHedgeState (Variables|Default|GetbIsUsed))
  (return true))

(fn GetItemName
  (return "None"))

(fn IsInventoryItem
  (return false))

(fn Pickup
  (params (Instigator :type Actor%20Object%20Reference))
  (return false))

(fn RecieveItem
  (params (ItemName :type Name :default "None"))
  (switch name ItemName
    (:FireStick
      (CallFunction|SetHedgeonFire)
      (return true true))
    (:Axe
      (CallFunction|StartDialogueSequence "RecieveItemHedgeAxe")
      (return false false))))