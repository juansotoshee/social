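; Campfire puzzle interactable for the ForestDemo scene that takes chopped wood, then a fire maker, then a frozen fish to cook.
; Received items go into its inventory component, which serves as the puzzle state for inspection dialogue and for wood, rubble and fire visuals, re-applied on gameplay load.
; After a cook delay, the fish mesh hides and the cooked fish item moves into its place.
; A timeline flickers the fire light from BeginPlay.
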(event Custom|CookFish
  (bind _fishmesh (Variables|Default|GetFishMesh))
  (bind _returnvalue (Transformation|GetWorldTransform _fishmesh))
  ;[0.5035 1 0.4828 0.3] Set the location of the cooked fish for the player.
  (Utilities|FlowControl|Delay (Variables|Default|GetCookDelay))
  (Development|SetHiddeninGame (Variables|Default|GetFishMesh) true false)
  (Transformation|SetActorLocationAndRotation (Variables|Default|GetCookedFishItemRef) (.location _returnvalue) (.rotation _returnvalue)))

(event Custom|SetActiveCookedFishLocation
  (bind _fishmesh (Variables|Default|GetFishMesh))
  (bind _returnvalue (Transformation|GetWorldTransform _fishmesh))
  ;[0.5035 1 0.4828 0.3] Set the location of the cooked fish for the player.
  (Development|SetHiddeninGame (Variables|Default|GetFishMesh) true false)
  (Transformation|SetActorLocationAndRotation (Variables|Default|GetCookedFishItemRef) (.location _returnvalue) (.rotation _returnvalue)))

(event EventBeginPlay
  (|CallParentFunction)
  ;[1 0.8888 0.4989 0.3] Animate a flicker effect for the fire light
  (Variables|Default|SetLightIntensity (Variables|/Script/Engine.LightComponentBase|GetIntensity (Variables|Components|GetFirePointLight)))
  (bind _brightness (Timeline|FireBrightness Play)
    (:Update
      (Rendering|Components|Light|SetIntensity (Variables|Components|GetFirePointLight) (* (Variables|Default|GetLightIntensity) _brightness)))))

(fn ConstructionScript
  (|CallParentFunction))

(fn OnInspection
  (params (Inspector :type Controller%20Object%20Reference))
  (if (Default|HasIteminInventory (Variables|Default|GetBP_InventoryComponent) "FireMaker")
    (CallFunction|StartDialogueSequence "InspectCampfireLit" Inspector)
    (elif (Default|HasIteminInventory (Variables|Default|GetBP_InventoryComponent) "ChoppedWood")
      (CallFunction|StartDialogueSequence "InspectCampfireUnlit" Inspector)
      (else
        (CallFunction|StartDialogueSequence "InspectCampfireWood" Inspector))))
  (return true))

(fn UpdateBonfireState
  (if (Variables|/Game/PNCTookit/Blueprints/Gameplay/Items/BP_ItemBase.BP_ItemBase_C|GetbIsActive (Variables|Default|GetCookedFishItemRef))
    (Rendering|SetVisibility (Variables|Default|GetWoodMesh) (Default|HasIteminInventory (Variables|Default|GetBP_InventoryComponent) "ChoppedWood") false)
    (if (Default|HasIteminInventory (Variables|Default|GetBP_InventoryComponent) "FireMaker")
      (if (Variables|/Game/PNCTookit/Blueprints/Gameplay/Items/BP_ItemBase.BP_ItemBase_C|GetbIsActive (Variables|Default|GetCookedFishItemRef))
        (Components|Activation|Activate (Variables|Components|GetFireParticle) true)
        (Rendering|SetVisibility (Variables|Default|GetBurntRubbleMesh) true false)
        (else
          (Components|Activation|Deactivate (Variables|Components|GetFireParticle) :!label _label)))
      (else
        (goto _label)))
    (if (Default|HasIteminInventory (Variables|Default|GetBP_InventoryComponent) "FrozenFish")
      (CallFunction|SetActiveCookedFishLocation))
    (else
      (Rendering|SetVisibility (Variables|Default|GetBurntRubbleMesh) false false)
      (Rendering|SetVisibility (Variables|Default|GetWoodMesh) false false)
      (Components|Activation|Deactivate (Variables|Components|GetFireParticle)))))

(fn LoadGameplayState
  (CallFunction|UpdateBonfireState)
  (return true))

(fn GetItemName
  (return "None"))

(fn IsInventoryItem
  (return false))

(fn Pickup
  (params (Instigator :type Actor%20Object%20Reference))
  (return false))

(fn RecieveItem
  (params (ItemName :type Name :default "None"))
  (bind _output_get (LocalVariables|SetItem ItemName))
  (switch name _output_get
    (:Default
      (return false false))
    (:ChoppedWood
      (Default|AddInventoryItem (Variables|Default|GetBP_InventoryComponent) (LocalVariables|GetItem))
      (CallFunction|UpdateBonfireState)
      (CallFunction|StartDialogueSequence "RecieveItemCampfireChoppedWood"))
    (:FireMaker
      (if (Default|HasIteminInventory (Variables|Default|GetBP_InventoryComponent) "ChoppedWood")
        (Default|AddInventoryItem (Variables|Default|GetBP_InventoryComponent) (LocalVariables|GetItem))
        (CallFunction|UpdateBonfireState)
        (CallFunction|StartDialogueSequence "RecieveItemCampfireFireMaker")
        (else
          (CallFunction|StartDialogueSequence "ReceiveItemFireMakerNoWood")
          (return false false))))
    (:FrozenFish
      (if (Default|HasIteminInventory (Variables|Default|GetBP_InventoryComponent) "FireMaker")
        (Default|AddInventoryItem (Variables|Default|GetBP_InventoryComponent) (LocalVariables|GetItem))
        (Development|SetHiddeninGame (Variables|Default|GetFishMesh) false false)
        (CallFunction|CookFish)
        (CallFunction|StartDialogueSequence "RecieveItemCampfireFish")
        (else
          (CallFunction|StartDialogueSequence "RecieveItemFishInvalid")
          (return false false))))
    (:StickHandle
      (CallFunction|StartDialogueSequence "RecieveItemCampfireHandleFailed")
      (return false false)))
  (return true true))