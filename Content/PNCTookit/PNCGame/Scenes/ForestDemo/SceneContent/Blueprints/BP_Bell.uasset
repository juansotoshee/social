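; BP_Bell is a one-shot usable bell in the PNC Toolkit forest demo that triggers the shopkeeper's introduction.
; Its UseObject function checks and clears IsActive, then casts the scene manager to BP_ForestDemoCaravan_SceneManager and calls ShopkeeperIntro.
; It then starts the UseBell dialogue sequence with itself as the initiating actor and returns false.
; The event graph and construction script add no behavior of their own.
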(event EventBeginPlay
  (|CallParentFunction) ; This node is disabled and will not be called.\nDrag off pins to build functionality.
)

(event Collision|EventActorBeginOverlap
  (params (OtherActor :type Actor%20Object%20Reference)))

(event EventTick
  (params (DeltaSeconds :type Float%20%28single-precision%29)))

(fn ConstructionScript
  (|CallParentFunction))

(fn UseObject
  (params (InteractingCharacter :type BP%20PNC%20Character%20Parent%20Object%20Reference))
  (if (Variables|Default|GetbIsActive)
    (Variables|Default|SetbIsActive false)
    (bind _asbp_forest_demo_caravan_scene_manager (Utilities|Casting|CastToBP_ForestDemoCaravan_SceneManager (CallFunction|GetSceneManager)))
    (Default|ShopkeeperIntro _asbp_forest_demo_caravan_scene_manager)
    (CallFunction|StartDialogueSequence "UseBell" self)
    (return false)))