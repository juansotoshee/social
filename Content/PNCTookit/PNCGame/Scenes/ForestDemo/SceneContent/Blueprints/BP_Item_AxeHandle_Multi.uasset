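; BP_Item_AxeHandle_Multi is a ForestDemo pickup item that acts as a limited supply of StickHandle items, allowing the player to hold one at a time.
; Its Pickup override runs the parent check, then checks the player controller's inventory and its own inventory component for StickHandle.
; It removes one from its own stock and returns that result, or plays the PickupStickFailed dialogue if the player has one or none remain.
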(event EventBeginPlay
  (|CallParentFunction) ; This node is disabled and will not be called.\nDrag off pins to build functionality.
)

(event Collision|EventActorBeginOverlap
  (params (OtherActor :type Actor%20Object%20Reference)))

(event EventTick
  (params (DeltaSeconds :type Float%20%28single-precision%29)))

(fn ConstructionScript
  (|CallParentFunction))

(fn Pickup
  (params (Instigator :type Actor%20Object%20Reference))
  (bind _success (|CallParentFunction Instigator))
  (if _success
    (if (Default|HasIteminInventory (Variables|/Game/PNCTookit/Blueprints/BP_PNCPlayerController.BP_PNCPlayerController_C|GetInventoryComponent (CallFunction|GetPNCPlayerController)) "StickHandle") ; Does the player already have a "Rock" item \nin their inventory?
      _
      (elif (Default|HasIteminInventory (Variables|Default|GetBP_InventoryComponent) "StickHandle") ; Does the "Pile Of Rocks" item still have rocks remaining?\n(haha, max the player can take is 2)
        (bind _return (Default|RemoveInventoryItem (Variables|Default|GetBP_InventoryComponent) "StickHandle" false))
        (return _return)
        (else
          _)))
    (CallFunction|StartDialogueSequence "PickupStickFailed")
    (return false)
    (else
      (return false))))