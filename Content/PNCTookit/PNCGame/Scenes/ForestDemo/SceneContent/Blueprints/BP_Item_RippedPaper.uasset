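; BP_Item_RippedPaper is a pickup item in the point-and-click toolkit's forest demo that is gated on talking to the shopkeeper.
; Its Pickup override calls the parent pickup only if the referenced shopkeeper has been spoken to.
; Otherwise it plays the PickupRubbishFailed dialogue sequence and returns false.
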(event EventBeginPlay
  (|CallParentFunction) ; This node is disabled and will not be called.\nDrag off pins to build functionality.
)

(event Collision|EventActorBeginOverlap
  (params (OtherActor :type Actor%20Object%20Reference)))

(event EventTick
  (params (DeltaSeconds :type Float%20%28single-precision%29)))

(fn ConstructionScript
  (|CallParentFunction))

(fn Pickup
  (params (Instigator :type Actor%20Object%20Reference))
  (if (Variables|/Game/PNCTookit/Blueprints/Characters/BP_PNCCharacter_Parent.BP_PNCCharacter_Parent_C|GetbIsSpokenTo (Variables|Default|GetShopKeeper%20Ref))
    (bind _success (|CallParentFunction (Variables|Default|GetInstigator)))
    (return _success)
    (else
      (CallFunction|StartDialogueSequence "PickupRubbishFailed")
      (return false))))