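; BP_Clock is an interactable point-and-click clock that cannot be picked up and answers interactions with dialogue rows.
; The first successful use sets IsUsed, and later uses play a different dialogue.
; Once used, inspection shows the current Now() time in a floating dialogue widget, guarded against duplicates and removed after three seconds.
; Any item given to it is accepted and consumed.
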(event Custom|DelayRemoveFloatingDialogue
  (Utilities|FlowControl|Delay 3.0)
  (Widget|RemovefromParent (Variables|Default|GetFloatingDialogueRef))
  (Variables|Default|SetFloatingDialogueRef 0))

(fn ConstructionScript
  (|CallParentFunction))

(fn UseObject
  (params (InteractingCharacter :type BP%20PNC%20Character%20Parent%20Object%20Reference))
  (bind _success (|CallParentFunction InteractingCharacter))
  (if _success
    (if (Variables|Default|GetbIsUsed)
      (CallFunction|StartDialogueSequence "UseClockOn" self)
      (else
        (Variables|Default|SetbIsUsed true)
        (CallFunction|StartDialogueSequence "UseClockOff" self))))
  (return _success))

(fn DisplayTimeDialogue
  (Variables|Default|GetFloatingDialogueRef
    (:then)
    (:else
      (bind _returnvalue (UserInterface|CreateWidget "/Game/PNCTookit/Blueprints/Gameplay/Dialogue/Widgets/WBP_FloatingDialogueText.WBP_FloatingDialogueText_C" 0 self 0 (Utilities|Struct|MakeSDialogueData (Utilities|Array|MakeArray "") (Utilities|Text|FormatText "The time is {time}" (Class|KismetTextLibrary|AsTimeDateTime (Math|DateTime|Now))) (Utilities|Array|MakeArray ""))))
      (bind _output_get (Variables|Default|SetFloatingDialogueRef _returnvalue))
      (UserInterface|Viewport|AddtoViewport _output_get 0)
      (CallFunction|DelayRemoveFloatingDialogue))))

(fn OnInspection
  (params (Inspector :type Controller%20Object%20Reference))
  (if (Variables|Default|GetbIsUsed)
    (CallFunction|DisplayTimeDialogue)
    (return true)
    (else
      (CallFunction|StartDialogueSequence "InspectClock" self)
      (return true))))

(fn GetItemName
  (return "None"))

(fn IsInventoryItem
  (return false))

(fn Pickup
  (params (Instigator :type Actor%20Object%20Reference))
  (CallFunction|StartDialogueSequence "PickupClockToHeavy" self)
  (return false))

(fn RecieveItem
  (params (ItemName :type Name :default "None"))
  (CallFunction|StartDialogueSequence "RecieveItemClockStorage" self)
  (return true true))