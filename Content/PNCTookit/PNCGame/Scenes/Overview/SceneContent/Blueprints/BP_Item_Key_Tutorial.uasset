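; BP_Item_Key_Tutorial is a key item variant that shows tutorial text through a pickup widget.
; On BeginPlay it creates a WBP_TutorialText from its TutorialText and assigns it to PickupWidget.
; Pickup and SetItemActiveState extend the parent logic to keep widget visibility in step with the item, hiding it once picked up.
; PlayPickupAnim skips the animation and immediately sets the item inactive.
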(event EventBeginPlay
  (|CallParentFunction)
  (bind _returnvalue (UserInterface|CreateWidget "/Game/PNCTookit/PNCGame/Scenes/Overview/SceneContent/Blueprints/WBP_TutorialText.WBP_TutorialText_C" 0 self (Variables|Default|GetTutorialText)))
  (UserInterface|SetWidget (Variables|Default|GetPickupWidget) _returnvalue))

(event EventPlayPickupAnim
  (params (Actor :type Actor%20Object%20Reference))
  ;[1 1 1] Skip the anim and go straight to setting the item as inactive (hidden)
  (CallFunction|SetItemActiveState false))

(fn ConstructionScript
  (|CallParentFunction))

(fn Pickup
  (params (Instigator :type Actor%20Object%20Reference))
  (bind _success (|CallParentFunction Instigator))
  (Rendering|SetVisibility (Variables|Default|GetPickupWidget) (not _success) false)
  (return _success))

(fn SetItemActiveState
  (params (bActive :type Boolean))
  (bind _return (|CallParentFunction bActive))
  (Rendering|SetVisibility (Variables|Default|GetPickupWidget) bActive false)
  (return _return))