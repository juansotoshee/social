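; BP_TutorialNotifier is an actor that displays tutorial text through its widget component in the PNC toolkit's overview scene.
; On BeginPlay it calls ShowNotifier with its ShowOnStartup setting.
; ShowNotifier either creates a new WBP_TutorialText from the actor's TutorialText, assigns it to the component and makes it visible, or hides the component.
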(event EventBeginPlay
  (CallFunction|ShowNotifier (Variables|Default|GetShowOnStartup)))

(fn ConstructionScript)

(fn ShowNotifier
  (params (Show :type Boolean))
  (if Show
    (bind _returnvalue (UserInterface|CreateWidget "/Game/PNCTookit/PNCGame/Scenes/Overview/SceneContent/Blueprints/WBP_TutorialText.WBP_TutorialText_C" 0 self (Variables|Default|GetTutorialText)))
    (UserInterface|SetWidget (Variables|Default|GetWidget) _returnvalue)
    (Rendering|SetVisibility (Variables|Default|GetWidget) true false)
    (else
      (Rendering|SetVisibility (Variables|Default|GetWidget) false false))))