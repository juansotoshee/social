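; BP_Log is an inspectable log for a point-and-click game that turns into a linked item when the player uses the axe on it.
; Inspection starts a dialogue, and it cannot be picked up.
; Receiving the axe activates the linked item at the log's location and rotation, then sets IsUsed, hiding the log and disabling its collision.
; Loading reapplies that state and repositions the item if the log was used.
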(fn ConstructionScript
  (|CallParentFunction))

(fn LoadGameplayState
  (bind _returnvalue (Transformation|GetActorTransform))
  (bind _bisused (Variables|Default|GetbIsUsed))
  (CallFunction|SetGameplayState _bisused)
  (if _bisused
    (Transformation|SetActorTransform (Variables|Default|GetItem) (Math|Transform|MakeTransform (.location _returnvalue) (.rotation _returnvalue) "1,1,1"))
    (return true)
    (else
      (return true))))

(fn OnAxeRecieved
  (bind _returnvalue (Transformation|GetActorTransform))
  ;[1 0.8448 0.5198 0.3] When the axe item is recieved, add chopped wood to the players inventory, set the gameplay state of the log, and run the given dialogue sequence.
  (bind _item (Variables|Default|GetItem)
    (:then
      (if (Variables|/Game/PNCTookit/Blueprints/Gameplay/Items/BP_ItemBase.BP_ItemBase_C|GetbIsActive _item)
        _
        (else
          (Default|SetItemActiveState (Variables|Default|GetItem) true)
          (Transformation|SetActorTransform (Variables|Default|GetItem) (Math|Transform|MakeTransform (.location _returnvalue) (.rotation _returnvalue) "1,1,1"))
          (CallFunction|SetGameplayState true))))
    (:else
      _))
  (return true))

(fn SetGameplayState
  (params (IsUsed :type Boolean))
  (bind _output_get (Variables|Default|SetbIsUsed IsUsed))
  (Rendering|SetActorHiddenInGame _output_get)
  (Collision|SetActorEnableCollision (not _output_get)))

(fn OnInspection
  (params (Inspector :type Controller%20Object%20Reference))
  (CallFunction|StartDialogueSequence "InspectLog" Inspector)
  (return false))

(fn GetItemName
  (return "None"))

(fn IsInventoryItem
  (return false))

(fn Pickup
  (params (Instigator :type Actor%20Object%20Reference))
  (return false))

(fn RecieveItem
  (params (ItemName :type Name :default "None"))
  (switch name ItemName
    (:Default
      (return false false))
    (:Axe
      (bind _return (CallFunction|OnAxeRecieved))
      (return _return _return))))