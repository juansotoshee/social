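; Interactable 3x3 sliding-tile puzzle that takes over view and input when used, with skip, reset and exit.
; CreateTiles spawns eight tiles into nine slots and randomly shuffles them, without a solvability check.
; SlideTile uses tile collision checks and the index array to find the empty slot, then lerps the tile there.
; Matching the winning order zooms out the camera, restores gameplay, records "MapSolved" and plays dialogue.
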(event Custom|OnFailed
  ;[0.5089 1 0.9734 0.298] Exit Puzzle
  (Puzzle|EndSlidePuzzle))

(event Custom|SlideTile
  (params (Tile :type BP%20Slide%20Tile%20Object%20Reference))
  ;[0.5089 1 0.9734 0.298] If valid, move selected tile to an available location
  (if (not (Variables|System|GetbAnimatingSlidingTile))
    (Variables|System|SetbAnimatingSlidingTile true)
    (bind _output_get (Variables|System|SetSlidingTileRef Tile))
    (bind (_location _return) (Helpers|FindValidMoveLocation (Variables|System|GetSlidingTileRef)))
    (if _return
      (bind _time (Timeline|Lerp PlayFromStart)
        (:Update
          (Transformation|SetActorTransform (Variables|System|GetSlidingTileRef) (Math|Transform|Lerp(Transform) (Transformation|GetActorTransform (Variables|System|GetSlidingTileRef)) (Helpers|GetGoalRelativeTransfrom _location) _time)))
        (:Finished
          (Math|Integer|IncrementInt (Variables|Puzzle|GetNumOfMoves)
            (:%20%20
              (Variables|System|SetbAnimatingSlidingTile false :!label _label)
              (bind _return_2 (Helpers|CheckTileOrder))
              (if _return_2
                (CallFunction|OnSuccess)
                (Variables|System|SetSlidingTileRef 0))))))
      (else
        (goto _label)))))

(event Custom|OnSuccess
  ;[0.5089 1 0.9734 0.298] On Puzzle Success
  (Puzzle|OnPuzzleCompletion)
  (Utilities|FlowControl|Sequence
    (:then_0
      ;[0.5089 1 0.9734 0.298] Play the camera 'Zoom out' animation when the puzzle has been completed
      (Variables|System|SetSpringArmStartingLength (Variables|/Script/Engine.SpringArmComponent|GetTargetArmLength (Variables|Default|GetSpringArm)))
      (bind _lerp (Timeline|Timeline_0 PlayFromStart)
        (:Update
          (Variables|/Script/Engine.SpringArmComponent|SetTargetArmLength (Variables|Default|GetSpringArm) (Math|Float|Lerp (Variables|System|GetSpringArmStartingLength) 2.5e+02 _lerp)))))
    (:then_1
      ;[0.5089 1 0.9734 0.298] After a short delay, end the puzzle.
      (Utilities|FlowControl|Delay 3.0)
      (Puzzle|EndSlidePuzzle)
      ;[0.5089 1 0.9734 0.298] After the puzzle has been solved, add state string to mark completion.
      (Default|AddStateStringtoScene (CallFunction|GetSceneManager) "" "MapSolved")
      ;[0.5089 1 0.9734 0.298] Completion dialogue.
      (Utilities|FlowControl|Delay 1.0)
      (CallFunction|StartDialogueSequence "SlidePuzzleComplete" self))))

(event EventResetPuzzle
  ;[0.5094 1 0.9701 0.3] Reset Puzzle
  (Puzzle|CreateTiles true)
  (Helpers|EnableCollisiononTiles true))

(event EventSkipPuzzle
  ;[0.5089 1 0.9734 0.298] Skip Puzzle
  (Puzzle|CreateTiles false)
  (Puzzle|OnPuzzleCompletion)
  (Utilities|FlowControl|Sequence
    (:then_0
      ;[0.5089 1 0.9734 0.298] Play the camera 'Zoom out' animation when the puzzle has been completed
      (Variables|System|SetSpringArmStartingLength (Variables|/Script/Engine.SpringArmComponent|GetTargetArmLength (Variables|Default|GetSpringArm)))
      (bind _lerp (Timeline|Timeline_0 PlayFromStart)
        (:Update
          (Variables|/Script/Engine.SpringArmComponent|SetTargetArmLength (Variables|Default|GetSpringArm) (Math|Float|Lerp (Variables|System|GetSpringArmStartingLength) 2.5e+02 _lerp)))))
    (:then_1
      ;[0.5089 1 0.9734 0.298] After a short delay, end the puzzle.
      (Utilities|FlowControl|Delay 3.0)
      (Puzzle|EndSlidePuzzle)
      ;[0.5089 1 0.9734 0.298] After the puzzle has been solved, add state string to mark completion.
      (Default|AddStateStringtoScene (CallFunction|GetSceneManager) "" "MapSolved")
      ;[0.5089 1 0.9734 0.298] Completion dialogue.
      (Utilities|FlowControl|Delay 1.0)
      (CallFunction|StartDialogueSequence "SlidePuzzleComplete" self))))

(event EventEndPuzzle
  ;[0.5089 1 0.9734 0.298] Exit Puzzle
  (Puzzle|EndSlidePuzzle))

(fn ConstructionScript
  (|CallParentFunction))

(fn UseObject
  (params (InteractingCharacter :type BP%20PNC%20Character%20Parent%20Object%20Reference))
  ;[0.9986 0.6641 1 0.3] Start the puzzle if the interaction is valid.
  (bind _success (|CallParentFunction InteractingCharacter))
  (if _success
    (Puzzle|StartSlidePuzzle)
    (CallFunction|StartDialogueSequence "UseSlidePuzzle" self)
    (return true)
    (else
      (return false))))

(fn FindValidMoveLocation
  (params (Tile :type BP%20Slide%20Tile%20Object%20Reference))
  (bind _tilesindexarray (Variables|Puzzle|GetTilesIndexArray))
  (bind _returnvalue (Utilities|Array|FindItem _tilesindexarray Tile))
  ;[1 0.679 0.3121 0.3] Find a valid move direction for the selected tile
  (for (_array_element _array_index) (Utilities|Array|MakeArray (Variables|/Game/PNCTookit/PNCGame/Scenes/Shared/Puzzles/Slide_Puzzle/BP_Slide_Tile.BP_Slide_Tile_C|GetCollision_Top Tile) (Variables|/Game/PNCTookit/PNCGame/Scenes/Shared/Puzzles/Slide_Puzzle/BP_Slide_Tile.BP_Slide_Tile_C|GetCollision_Bottom Tile) (Variables|/Game/PNCTookit/PNCGame/Scenes/Shared/Puzzles/Slide_Puzzle/BP_Slide_Tile.BP_Slide_Tile_C|GetCollision_Left Tile) (Variables|/Game/PNCTookit/PNCGame/Scenes/Shared/Puzzles/Slide_Puzzle/BP_Slide_Tile.BP_Slide_Tile_C|GetCollision_Right Tile))
    (if (not (Default|IsColliding Tile _array_element))
      (LocalVariables|SetDirection (Utilities|Array|Get(acopy) (Utilities|Array|MakeArray "NewEnumerator0" "NewEnumerator3" "NewEnumerator6" "NewEnumerator7") _array_index))
      (LocalVariables|SetOldIndex _returnvalue)
      (LocalVariables|SetNewIndex (Utilities|Select :Index (LocalVariables|GetDirection) :NewEnumerator8 0 :NewEnumerator0 (+ _returnvalue -3) :NewEnumerator1 0 :NewEnumerator2 0 :NewEnumerator3 (+ _returnvalue 3) :NewEnumerator4 0 :NewEnumerator5 0 :NewEnumerator6 (+ _returnvalue -1) :NewEnumerator7 (+ _returnvalue 1)))
      (Utilities|IsValid (Utilities|Array|Get(acopy) (Variables|Puzzle|GetTilesIndexArray) (LocalVariables|GetNewIndex))
        (:Is%20Not%20Valid
          (Utilities|Array|SetArrayElem (Variables|Puzzle|GetTilesIndexArray) (LocalVariables|GetNewIndex) Tile)
          (Utilities|Array|SetArrayElem (Variables|Puzzle|GetTilesIndexArray) (LocalVariables|GetOldIndex) 0)
          (return (Utilities|Array|Get(acopy) (Variables|System|GetRelativeLocations) (LocalVariables|GetNewIndex)) true)))))
  (return "0, 0, 0" false))

(fn CreateTiles
  (params (ShuffleTiles :type Boolean))
  (bind _tilelocation_5 (Variables|Default|GetTileLocation_5))
  (bind _tilelocation_2 (Variables|Default|GetTileLocation_2))
  (bind _tilelocation_3 (Variables|Default|GetTileLocation_3))
  (bind _tilelocation_4 (Variables|Default|GetTileLocation_4))
  (bind _tilelocation_1 (Variables|Default|GetTileLocation_1))
  (bind _tilelocation_6 (Variables|Default|GetTileLocation_6))
  (bind _tilelocation_7 (Variables|Default|GetTileLocation_7))
  (bind _tilelocation_8 (Variables|Default|GetTileLocation_8))
  (bind _tilelocation_9 (Variables|Default|GetTileLocation_9))
  (bind _array (Utilities|Array|MakeArray _tilelocation_1 _tilelocation_2 _tilelocation_3 _tilelocation_4 _tilelocation_5 _tilelocation_6 _tilelocation_7 _tilelocation_8 _tilelocation_9))
  (bind _returnvalue (Utilities|Array|Length _array))
  (bind _returnvalue_2 (- _returnvalue 1))
  ;[0.5212 1 0.4733 0.3] Create puzzle tiles and set their location on the board
  (Variables|Puzzle|SetNumOfMoves 0)
  (Utilities|Array|Clear (Variables|System|GetRelativeLocations))
  (Utilities|Array|Clear (Variables|Puzzle|GetWinningTilesArray))
  (if (>= (Utilities|Array|Length (Variables|Puzzle|GetTilesIndexArray)) 1)
    (for _array_element (Variables|Puzzle|GetTilesIndexArray)
      (Utilities|IsValid _array_element
        (:Is%20Valid
          (Actor|DestroyActor _array_element))))
    (Utilities|Array|Clear (Variables|Puzzle|GetTilesIndexArray)))
  (for (_array_element_2 _array_index) _array
    (Utilities|Array|Add (Variables|System|GetRelativeLocations) (Variables|/Script/Engine.SceneComponent|GetRelativeLocation _array_element_2))
    (if (< _array_index _returnvalue_2)
      (bind _returnvalue_3 (Game|SpawnActorfromClass "/Game/PNCTookit/PNCGame/Scenes/Shared/Puzzles/Slide_Puzzle/BP_Slide_Tile.BP_Slide_Tile_C" (Helpers|GetGoalRelativeTransfrom (Variables|/Script/Engine.SceneComponent|GetRelativeLocation _array_element_2)) "Undefined" 0 0))
      (Utilities|Array|Add (Variables|Puzzle|GetWinningTilesArray) _returnvalue_3)
      (Utilities|Array|Add (Variables|Puzzle|GetTilesIndexArray) _returnvalue_3)
      (Default|InitTile _returnvalue_3 self _array_index)))
  (Utilities|Array|SetArrayElem (Variables|Puzzle|GetTilesIndexArray) _returnvalue_2 0 true)
  (if ShuffleTiles
    (Helpers|ShuffleTileArray)))

(fn ShuffleTileArray
  ;[0.5021 0.869 1 0.3] Shuffle the order of the tiles
  (Utilities|Array|Shuffle (Variables|Puzzle|GetTilesIndexArray))
  (for (_array_element _array_index) (Variables|System|GetRelativeLocations)
    (Utilities|IsValid (Utilities|Array|Get(acopy) (Variables|Puzzle|GetTilesIndexArray) _array_index)
      (:Is%20Valid
        (Transformation|SetActorTransform (Utilities|Array|Get(acopy) (Variables|Puzzle|GetTilesIndexArray) _array_index) (Helpers|GetGoalRelativeTransfrom _array_element) false true)))))

(fn GetGoalRelativeTransfrom
  (params (Relative%20Location :type Vector))
  (bind _returnvalue (Transformation|GetActorRotation))
  (return (Math|Transform|MakeTransform (+ (Math|Vector|RotateVector Relative%20Location _returnvalue) (Transformation|GetActorLocation)) _returnvalue)))

(fn CheckTileOrder
  (for (_array_element _array_index) (Variables|Puzzle|GetWinningTilesArray)
    (if (not (== _array_element (Utilities|Array|Get(acopy) (Variables|Puzzle|GetTilesIndexArray) _array_index)))
      (return false)))
  (return true))

(fn EnableCollisiononTiles
  (params (Enable :type Boolean))
  (for _array_element (Variables|Puzzle|GetTilesIndexArray)
    (Utilities|IsValid _array_element
      (:Is%20Valid
        (Collision|SetActorEnableCollision _array_element Enable)))))

(fn LoadGameplayState
  ;[0.9404 0.7396 1 0.3] Load the Gameplay state of the
  (if (Variables|Default|GetbIsUsed)
    (Puzzle|CreateTiles false)
    (else
      (Puzzle|CreateTiles true)))
  (return true))

(fn OnPuzzleCompletion
  ;[0.4769 0.8897 1 0.3] On Completion remove the Puzzle UI and set the completion state
  (Variables|Default|SetbIsActive false)
  (Variables|Default|SetbIsUsed true)
  (Utilities|IsValid (Variables|System|GetSlidePuzzleWidget)
    (:Is%20Valid
      (Widget|RemovefromParent (Variables|System|GetSlidePuzzleWidget))
      (Variables|System|SetSlidePuzzleWidget 0))
    (:Is%20Not%20Valid
      _))
  (for _array_element (Variables|Puzzle|GetTilesIndexArray)
    (Utilities|IsValid _array_element
      (:Is%20Valid
        (Collision|SetActorEnableCollision _array_element false)))))

(fn StartSlidePuzzle
  ;[1 0.6192 0.4366 0.3] Set Player and Puzzle state
  (Default|SetInputProfile (CallFunction|GetPNCPlayerController) "Puzzle")
  (Collision|SetCollisionResponsetoChannel (Variables|/Script/Engine.Character|GetCapsuleComponent (CallFunction|GetPNCCharacter)) "ECC_Visibility" "ECR_Ignore")
  (Rendering|SetActorHiddenInGame (CallFunction|GetPNCCharacter) true)
  (Game|Player|SetViewTargetwithBlend (CallFunction|GetPNCPlayerController) self 1.0 "VTBlend_EaseInOut" 2.0 false)
  (Helpers|EnableCollisiononTiles true)
  (bind _returnvalue (UserInterface|CreateWidget "/Game/PNCTookit/PNCGame/Scenes/Shared/Puzzles/Slide_Puzzle/WBP_Slide_Puzzle_UI.WBP_Slide_Puzzle_UI_C" 0 self))
  (bind _output_get (Variables|System|SetSlidePuzzleWidget _returnvalue))
  (UserInterface|Viewport|AddtoViewport _output_get 15))

(fn EndSlidePuzzle
  (bind _slidepuzzlewidget (Variables|System|GetSlidePuzzleWidget))
  ;[1 0.7936 0.4853] End Puzzle
  (Utilities|IsValid _slidepuzzlewidget
    (:Is%20Valid
      (Widget|RemovefromParent _slidepuzzlewidget))
    (:Is%20Not%20Valid
      _))
  (Default|SetInputProfile (CallFunction|GetPNCPlayerController) "Gameplay")
  (Rendering|SetActorHiddenInGame (CallFunction|GetPNCCharacter) false)
  (Game|Player|SetViewTargetwithBlend (CallFunction|GetPNCPlayerController) (Variables|/Game/PNCTookit/Blueprints/BP_PNCPlayerController.BP_PNCPlayerController_C|GetCameraManagerRef (CallFunction|GetPNCPlayerController)) 1.0 "VTBlend_Cubic" 0.0 false)
  (Collision|SetCollisionResponsetoChannel (Variables|/Script/Engine.Character|GetCapsuleComponent (CallFunction|GetPNCCharacter)) "ECC_Visibility" "ECR_Block"))

(fn ReturnPuzzleResult
  (params (Success :type Boolean))
  (if Success
    (CallFunction|OnSuccess)
    (else
      (CallFunction|OnFailed)))
  (return true))