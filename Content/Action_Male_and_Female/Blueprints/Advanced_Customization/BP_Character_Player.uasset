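; Player character Blueprint that extends its parent's customization events to update the visible body and weapon meshes.
; Gender changes look up the active customization key in DT_Genders and apply that row's skeletal mesh and matching animation Blueprint.
; Weapon changes and show-in-game toggles fill SKMWeapon from the active DT_Weapons row, or clear it when the weapon is hidden.
; Each override calls its parent first, keeping the default behavior.
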(event EventOnShowWeaponinGame
  (params (bShowWeapon :type Boolean))
  (|CallParentFunction bShowWeapon)
  (if bShowWeapon
    ;[1 1 1] Apply the current Weapon Mesh
    (bind _returnvalue (Utilities|GetDataTableRow "/Game/Action_Male_and_Female/DataTables/Weapons/DT_Weapons.DT_Weapons" (CallFunction|GetActiveCustomizationbyKey "Weapon"))
      (:then
        (Class|SkinnedMeshComponent|SetSkeletalMesh (Variables|Default|GetSKM_Weapon) (Utilities|Struct|BreakFWeapons _returnvalue) true)))
    (else
      ;[1 1 1] Clear the mesh again
      (Class|SkinnedMeshComponent|SetSkeletalMesh (Variables|Default|GetSKM_Weapon) 0 true))))

(event EventOnWeaponChanged
  (params (NewWeapon :type Name :default "None"))
  (|CallParentFunction NewWeapon)
  ;[1 1 1] Check if the weapon should be visible
  (if (Variables|Default|GetbShowWeaponInGame)
    ;[1 1 1] Apply the new Weapon Mesh
    (bind _returnvalue (Utilities|GetDataTableRow "/Game/Action_Male_and_Female/DataTables/Weapons/DT_Weapons.DT_Weapons" (CallFunction|GetActiveCustomizationbyKey "Weapon"))
      (:then
        (Class|SkinnedMeshComponent|SetSkeletalMesh (Variables|Default|GetSKM_Weapon) (Utilities|Struct|BreakFWeapons _returnvalue) true)))
    (else
      ;[1 1 1] Clear the mesh otherwise
      (Class|SkinnedMeshComponent|SetSkeletalMesh (Variables|Default|GetSKM_Weapon) 0 true))))

(event EventOnGenderChanged
  (params (NewGender :type Name :default "None"))
  ;[1 1 1] In addition to the default changes, also apply a new mesh and animation blueprint matching the mesh
  (|CallParentFunction NewGender)
  (bind _returnvalue (Utilities|GetDataTableRow "/Game/Action_Male_and_Female/DataTables/Genders/DT_Genders.DT_Genders" (CallFunction|GetActiveCustomizationbyKey "Gender"))
    (:then
      (Class|SkinnedMeshComponent|SetSkeletalMesh (Variables|Character|GetMesh) (.Mesh (Utilities|Struct|BreakFGenders _returnvalue)) false)
      (Class|SkeletalMeshComponent|SetAnimClass (Variables|Character|GetMesh) (.AnimationBlueprint (Utilities|Struct|BreakFGenders _returnvalue))))))

(fn ConstructionScript)